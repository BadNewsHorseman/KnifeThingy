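; BP_GameMode is a game mode that keeps the score.
; Its AddPoints event adds the passed amount to Points, then stores that amount plus five in PointsToGrant.
; SelectColor, BeginPlay and Tick are empty.
; Unconnected nodes would give the first BP_Wheel a random color from AvailableColors, print the color and score, and call SelectColor, but none of them run.
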(event `AddPoints`
  (params (Pointstogrant :type Integer))
  (set `self.Points` (+ (`self.Points`) Pointstogrant))
  (set `self.PointsToGrant` (+ Pointstogrant 5)))

(event `SelectColor`
  (params (NewParam :type "Actor Object Reference")))

(event `self.ReceiveBeginPlay`)

(event `self.ReceiveTick`
  (params (DeltaSeconds :type "Float (single-precision)")))

(fn `UserConstructionScript`)