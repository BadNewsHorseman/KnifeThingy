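; BP_Attack is an actor that performs a one-time lightning effect while rising through the world.
; While its Attack flag is true, Tick moves it up the Z axis at Speed, scaled by delta time, without sweeping.
; A DoOnce gate spawns a lightning emitter at its location, then after a short delay plays a 2D sound and destroys the emitter.
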(event `self.ReceiveTick`
  (params (DeltaSeconds :type "Float (single-precision)"))
  (bind _returnvalue (`self.K2_GetActorLocation`))
  (if (`self.Attack`)
    (`self.K2_SetActorLocation` (`KismetMathLibrary.MakeVector` (.x _returnvalue) (.y _returnvalue) (+ (.z _returnvalue) (* DeltaSeconds (`self.Speed`)))))
    (`/Engine/EditorBlueprintResources/StandardMacros.DoOnce` false
      (:`Completed`
        (bind _returnvalue_2 (`GameplayStatics.SpawnEmitterAtLocation` "/Game/Cartoony_Impact_-_Stylized_Particle_Simulation_1/Particles/PS_Lightning2.PS_Lightning2" _returnvalue))
        (`KismetSystemLibrary.Delay` 1.0)
        (`GameplayStatics.PlaySound2D` null 1.0 1.0 0.0 null null)
        (`ActorComponent.K2_DestroyComponent` _returnvalue_2)))))

(fn `UserConstructionScript`)