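; BP_Wheel4 is a four-box colour wheel target that scores BP_Attack hits against a random target colour.
; BeginPlay blocks wheel spawning, then loops over PointsToGrant, adding HUD balls and re-rolling the colour shown as Colortohit.
; Box overlaps add or subtract points by colour match (box names mostly differ from colours checked), destroy the attack and remove a ball icon.
; When no balls remain, it re-enables spawning and flags itself as Wheeltokill.
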(event `AddPoints`)

(event `self.ReceiveBeginPlay`
  (bind _colors (`self.colors`))
  (bind _hudref (`/Game/BP_GameMode.HUDREF` (`self.GameModeRef`)))
  (bind _hudref_2 (`/Game/BP_GameMode.HUDREF` (`self.GameModeRef`)))
  (set `/Game/BP_GameMode.canspawnwheel` false (`self.GameModeRef`))
  (bind _asbp_game_mode (cast `/Game/BP_GameMode` (`GameplayStatics.GetGameMode`)))
  (for _ (range (`/Game/BP_GameMode.PointsToGrant` _asbp_game_mode))
    (`/Game/UI_HUD.addtoballs` _hudref_2 (`/Game/UI_HUD.img_ball` _hudref_2))
    (bind _output_get (set `self.Color` (`|GetArrayItem` _colors (`KismetMathLibrary.RandomIntegerInRange` 0 (`KismetArrayLibrary.Array_Length` _colors)))))
    (switch `string` _output_get
      (:`purple`
        (set `/Game/UI_HUD.colortohit` (`self.purple`) _hudref)
        (bind _asbp_game_mode_2 (cast `/Game/BP_GameMode` (`GameplayStatics.GetGameMode`)))
        (set `self.GameModeRef` _asbp_game_mode_2))
      (:`red`
        (set `/Game/UI_HUD.colortohit` (`self.red`) _hudref)
        (bind _asbp_game_mode_3 (cast `/Game/BP_GameMode` (`GameplayStatics.GetGameMode`)))
        (set `self.GameModeRef` _asbp_game_mode_3))
      (:`blue`
        (set `/Game/UI_HUD.colortohit` (`self.blue`) _hudref)
        (bind _asbp_game_mode_4 (cast `/Game/BP_GameMode` (`GameplayStatics.GetGameMode`)))
        (set `self.GameModeRef` _asbp_game_mode_4))
      (:`lightblue`
        (set `/Game/UI_HUD.colortohit` (`self.lightblue`) _hudref)
        (bind _asbp_game_mode_5 (cast `/Game/BP_GameMode` (`GameplayStatics.GetGameMode`)))
        (set `self.GameModeRef` _asbp_game_mode_5)))))

(event `self.BoxLightBlue.OnComponentBeginOverlap`
  (params (OverlappedComponent :type "PrimitiveComponent Object Reference") (OtherActor :type "Actor Object Reference") (OtherComp :type "PrimitiveComponent Object Reference") (OtherBodyIndex :type Integer) (bFromSweep :type Boolean) (SweepResult :type "HitResult Structure (by ref)"))
  (bind _gamemoderef (`self.GameModeRef`))
  (bind _gamemoderef_2 (`self.GameModeRef`))
  (if (== (`self.Color`) "purple")
    (bind _asbp_attack (cast `/Game/BP_Attack` OtherActor))
    (`/Game/BP_GameMode.AddPoints` _gamemoderef (`self.pointstogrant`))
    (`self.K2_DestroyActor` _asbp_attack)
    (else
      (bind _asbp_attack_2 (cast `/Game/BP_Attack` OtherActor))
      (`/Game/BP_GameMode.AddPoints` _gamemoderef (* (`self.pointstogrant`) -1))
      (`self.K2_DestroyActor` _asbp_attack_2)))
  (`PanelWidget.RemoveChildAt` (`/Game/UI_HUD.balls_amt` (`/Game/BP_GameMode.HUDREF` _gamemoderef_2)) 0 :!label _label)
  (if (not (> (`/Game/BP_GameMode.ballsleft` (`self.GameModeRef`)) 0))
    (set `/Game/BP_GameMode.canspawnwheel` true _gamemoderef_2)
    (set `/Game/BP_GameMode.wheeltokill` self (`self.GameModeRef`))))

(event `self.BoxBlue.OnComponentBeginOverlap`
  (params (OverlappedComponent :type "PrimitiveComponent Object Reference") (OtherActor :type "Actor Object Reference") (OtherComp :type "PrimitiveComponent Object Reference") (OtherBodyIndex :type Integer) (bFromSweep :type Boolean) (SweepResult :type "HitResult Structure (by ref)"))
  (bind _gamemoderef (`self.GameModeRef`))
  (if (== (`self.Color`) "blue")
    (bind _asbp_attack (cast `/Game/BP_Attack` OtherActor))
    (`/Game/BP_GameMode.AddPoints` _gamemoderef (`self.pointstogrant`))
    (`self.K2_DestroyActor` _asbp_attack)
    (goto _label)
    (else
      (bind _asbp_attack_2 (cast `/Game/BP_Attack` OtherActor))
      (`/Game/BP_GameMode.AddPoints` _gamemoderef (* (`self.pointstogrant`) -1))
      (`self.K2_DestroyActor` _asbp_attack_2)
      (goto _label))))

(event `self.BoxRed.OnComponentBeginOverlap`
  (params (OverlappedComponent :type "PrimitiveComponent Object Reference") (OtherActor :type "Actor Object Reference") (OtherComp :type "PrimitiveComponent Object Reference") (OtherBodyIndex :type Integer) (bFromSweep :type Boolean) (SweepResult :type "HitResult Structure (by ref)"))
  (bind _gamemoderef (`self.GameModeRef`))
  (bind _pointstogrant (`self.pointstogrant`))
  (if (== (`self.Color`) "lightblue")
    (bind _asbp_attack (cast `/Game/BP_Attack` OtherActor))
    (`/Game/BP_GameMode.AddPoints` _gamemoderef _pointstogrant)
    (`self.K2_DestroyActor` _asbp_attack)
    (goto _label)
    (else
      (bind _asbp_attack_2 (cast `/Game/BP_Attack` OtherActor))
      (`/Game/BP_GameMode.AddPoints` _gamemoderef (* _pointstogrant -1))
      (`self.K2_DestroyActor` _asbp_attack_2)
      (goto _label))))

(event `self.BoxPurple.OnComponentBeginOverlap`
  (params (OverlappedComponent :type "PrimitiveComponent Object Reference") (OtherActor :type "Actor Object Reference") (OtherComp :type "PrimitiveComponent Object Reference") (OtherBodyIndex :type Integer) (bFromSweep :type Boolean) (SweepResult :type "HitResult Structure (by ref)"))
  (bind _pointstogrant (`self.pointstogrant`))
  (bind _gamemoderef (`self.GameModeRef`))
  (if (== (`self.Color`) "red")
    (bind _asbp_attack (cast `/Game/BP_Attack` OtherActor))
    (`/Game/BP_GameMode.AddPoints` _gamemoderef _pointstogrant)
    (`self.K2_DestroyActor` _asbp_attack)
    (goto _label)
    (else
      (bind _asbp_attack_2 (cast `/Game/BP_Attack` OtherActor))
      (`/Game/BP_GameMode.AddPoints` _gamemoderef (* _pointstogrant -1))
      (`self.K2_DestroyActor` _asbp_attack_2)
      (goto _label))))

(fn `UserConstructionScript`)